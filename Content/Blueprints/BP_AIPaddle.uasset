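; AI-controlled Pong paddle pawn that moves vertically to intercept the ball and plays a sound when the ball hits it.
; On Tick, only while the ball's Z velocity is positive, it linearly extrapolates the ball's Z at the paddle's Y, ignoring bounces, and steers toward it.
; MovePaddle applies scaled movement input and stores the direction, exposed through GetZVelocity.
; The ball reference is supplied through SetGameBallReference.
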(event `self.ReceiveTick`
  (params (DeltaSeconds :type "Float (single-precision)"))
  (bind _z (.z (`self.K2_GetActorLocation`)))
  (if (> (.z (`self.GetVelocity` (`self.GameBall`))) 0.0)
    (bind _zcoordinate (`self.ComputeBallZCoordinate`))
    (if (> _zcoordinate _z)
      (`self.MovePaddle` 1.0)
      (elif (< _zcoordinate _z)
        (`self.MovePaddle` -1.0)
        (else
          (`self.MovePaddle` 0.0))))))

(event `self.CollisionComponent.OnComponentHit`
  (params (HitComponent :type "PrimitiveComponent Object Reference") (OtherActor :type "Actor Object Reference") (OtherComp :type "PrimitiveComponent Object Reference") (NormalImpulse :type "Vector Structure") (Hit :type "HitResult Structure (by ref)"))
  (cast `/Game/Blueprints/BP_Ball` OtherActor)
  (`GameplayStatics.PlaySoundAtLocation` "/Game/Effects/pong-paddle.pong-paddle" (`self.K2_GetActorLocation`) (struct) 1.0 1.0 0.0 null null null))

(fn `ComputeBallZCoordinate`
  (returns (ZCoordinate :type "Float (double-precision)"))
  (bind _gameball (`self.GameBall`))
  (return (+ (.z (`self.K2_GetActorLocation` _gameball)) (* (/ (- (.y (`self.K2_GetActorLocation`)) (.y (`self.K2_GetActorLocation` _gameball))) (.y (`self.GetVelocity` _gameball))) (.z (`self.GetVelocity` _gameball))))))

(fn `GetZVelocity`
  (returns (ZVelocity :type "Float (double-precision)"))
  (return (`self.ZVelocity`)))

(fn `MovePaddle`
  (params (AxisValue :type "Float (double-precision)"))
  (set `self.ZVelocity` AxisValue)
  (`self.AddMovementInput` (`KismetMathLibrary.MakeVector` 0.0 0.0 (* AxisValue (`self.Scale`)))))

(fn `SetGameBallReference`
  (params (Ball :type "/Game/Blueprints/BP_Ball Object Reference"))
  (set `self.GameBall` Ball))

(fn `UserConstructionScript`)