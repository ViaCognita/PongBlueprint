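; BP_Ball is the ball in a Pong-style game, moved by a ProjectileMovementComponent that drives its query-only collision component.
; Paddle hits send it along Y away from that paddle using the paddle's Z velocity, while other hits flip Z; SetRandomZVelocity replaces zero Z with a random vertical kick.
; Overlapping goals named Goal_AI or Goal_Player adds the matching point in BP_GameState.
; FireInDirection and StopMovement launch and halt it.
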(event `self.CollisionComponent.OnComponentHit`
  (params (HitComponent :type "PrimitiveComponent Object Reference") (OtherActor :type "Actor Object Reference") (OtherComp :type "PrimitiveComponent Object Reference") (NormalImpulse :type "Vector Structure") (Hit :type "HitResult Structure (by ref)"))
  (bind _projectilemovementcomponent (`self.ProjectileMovementComponent`))
  (bind _returnvalue (`MovementComponent.GetMaxSpeed` _projectilemovementcomponent))
  (bind _asbp_paddle (cast `/Game/Blueprints/BP_Paddle` OtherActor)
    (:`then`
      (bind _zvelocity (`/Game/Blueprints/BP_Paddle.GetZVelocity` _asbp_paddle))
      (bind _reflectedvelocityfixed (`self.SetRandomZVelocity` (* (`KismetMathLibrary.MakeVector` 0.0 1.0 _zvelocity) _returnvalue)))
      (set `MovementComponent.Velocity` _reflectedvelocityfixed (`self.ProjectileMovementComponent`))
      (`KismetSystemLibrary.PrintString` (`KismetStringLibrary.Conv_VectorToString` _reflectedvelocityfixed) true true (struct :`G` 0.66 :`B` 1.0 :`A` 1.0) 4.0))
    (:`CastFailed`
      (bind _asbp_aipaddle (cast `/Game/Blueprints/BP_AIPaddle` OtherActor)
        (:`then`
          (bind _zvelocity_2 (`/Game/Blueprints/BP_AIPaddle.GetZVelocity` _asbp_aipaddle))
          (bind _reflectedvelocityfixed_2 (`self.SetRandomZVelocity` (* (`KismetMathLibrary.MakeVector` 0.0 -1.0 _zvelocity_2) _returnvalue)))
          (set `MovementComponent.Velocity` _reflectedvelocityfixed_2 (`self.ProjectileMovementComponent`))
          (`KismetSystemLibrary.PrintString` (`KismetStringLibrary.Conv_VectorToString` _reflectedvelocityfixed_2) true true (struct :`G` 0.66 :`B` 1.0 :`A` 1.0) 4.0))
        (:`CastFailed`
          (bind _output_get (set `self.ReflectedVelocity` (`KismetMathLibrary.MakeVector` (.x (`MovementComponent.Velocity` _projectilemovementcomponent)) (.y (`MovementComponent.Velocity` _projectilemovementcomponent)) (* -1 (.z (`MovementComponent.Velocity` _projectilemovementcomponent))))))
          (bind _reflectedvelocityfixed_3 (`self.SetRandomZVelocity` _output_get))
          (set `MovementComponent.Velocity` _reflectedvelocityfixed_3 (`self.ProjectileMovementComponent`))
          (`KismetSystemLibrary.PrintString` (`KismetStringLibrary.Conv_VectorToString` _reflectedvelocityfixed_3) true true (struct :`G` 0.66 :`B` 1.0 :`A` 1.0) 4.0))))))

(event `self.CollisionComponent.OnComponentBeginOverlap`
  (params (OverlappedComponent :type "PrimitiveComponent Object Reference") (OtherActor :type "Actor Object Reference") (OtherComp :type "PrimitiveComponent Object Reference") (OtherBodyIndex :type Integer) (bFromSweep :type Boolean) (SweepResult :type "HitResult Structure (by ref)"))
  (bind _returnvalue (`KismetSystemLibrary.GetObjectName` OtherActor))
  (bind _returnvalue_2 (`GameplayStatics.GetGameState`))
  (if (`KismetStringLibrary.EqualEqual_StrStr` _returnvalue "Goal_AI")
    (bind _asbp_game_state (cast `/Game/Blueprints/BP_GameState` _returnvalue_2))
    (`/Game/Blueprints/BP_GameState.AddAIPoint` _asbp_game_state)
    (elif (`KismetStringLibrary.EqualEqual_StrStr` _returnvalue "Goal_Player")
      (bind _asbp_game_state_2 (cast `/Game/Blueprints/BP_GameState` _returnvalue_2))
      (`/Game/Blueprints/BP_GameState.AddPlayerPoint` _asbp_game_state_2))))

(fn `FireInDirection`
  (params (ShootDirection :type "Vector Structure"))
  (bind _projectilemovementcomponent (`self.ProjectileMovementComponent`))
  (set `MovementComponent.Velocity` (* ShootDirection (`MovementComponent.GetMaxSpeed` _projectilemovementcomponent)) _projectilemovementcomponent))

(fn `SetRandomZVelocity`
  (params (ReflectedVelocity :type "Vector Structure"))
  (returns (ReflectedVelocityFixed :type "Vector Structure"))
  (bind _x (.x ReflectedVelocity))
  (if (== 0.0 (.z ReflectedVelocity))
    (if (`KismetMathLibrary.RandomBool`)
      (return (`KismetMathLibrary.MakeVector` _x (.y ReflectedVelocity) (* 1 (`ProjectileMovementComponent.MaxSpeed` (`self.ProjectileMovementComponent`)))))
      (else
        (return (`KismetMathLibrary.MakeVector` _x _x (* -1 (`ProjectileMovementComponent.MaxSpeed` (`self.ProjectileMovementComponent`)))))))
    (else
      (return ReflectedVelocity))))

(fn `StopMovement`
  (set `MovementComponent.Velocity` (`KismetMathLibrary.Vector_Zero`) (`self.ProjectileMovementComponent`)))

(fn `UserConstructionScript`
  ;[1 1 1] Collision configuration section
  (`PrimitiveComponent.SetCollisionEnabled` (`self.VisualComponent`) "NoCollision") ; Disable collisions in Visual Component.
  (`PrimitiveComponent.SetCollisionEnabled` (`self.CollisionComponent`) "QueryOnly") ; Enable Query Only Collisions in the Collision component.
  (`PrimitiveComponent.SetCollisionObjectType` (`self.CollisionComponent`) "ECC_GameTraceChannel1") ; Set collision object type to Projectile.
  (`PrimitiveComponent.SetCollisionResponseToAllChannels` (`self.CollisionComponent`) "ECR_Ignore") ; Set response to all channels to ignore.
  (`PrimitiveComponent.SetCollisionResponseToChannel` (`self.CollisionComponent`) "ECC_Pawn" "ECR_Block") ; Set block response to Pawn's object channel.
  (`PrimitiveComponent.SetCollisionResponseToChannel` (`self.CollisionComponent`) "ECC_GameTraceChannel2" "ECR_Block") ; Set block response to Edge's object channel.
  (`PrimitiveComponent.SetCollisionResponseToChannel` (`self.CollisionComponent`) "ECC_GameTraceChannel3" "ECR_Overlap") ; Set overlap response to Point's object channel.
  (set `PrimitiveComponent.bGenerateOverlapEvents` true (`self.CollisionComponent`)) ; Set to generate overlap events.
  (`MovementComponent.SetUpdatedComponent` (`self.ProjectileMovementComponent`) (`self.CollisionComponent`)) ; Use this component to drive ball's movement.
)