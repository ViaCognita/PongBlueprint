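; Game state for a paddle-and-ball match against an AI, tracking both scores until one side reaches MaxScore.
; StartGame spawns the ball and finds both paddles on first start, otherwise resets scores and paddle positions, then launches the ball based on LastScore.
; Point functions update score, reset the ball and check for game end; the player's also update UI.
; GameEnded shows an end menu with the result and switches to UI-only input.
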(fn `AddAIPoint`
  (bind _output_get (set `self.AIScore` (+ (`self.AIScore`) 1)))
  (set `self.LastScore` "NewEnumerator1")
  (`/Game/Blueprints/Widgets/UI/UMG_PlayerHUD.UpdateAIScore` (`/Game/Blueprints/BP_Paddle.PlayerUIRef` (`self.PlayerPaddle`)) _output_get)
  (`self.ResetTheBall`)
  (bind _isended (`self.IsGameEnded`))
  (if _isended
    (`self.GameEnded`)))

(fn `AddPlayerPoint`
  (bind _output_get (set `self.PlayerScore` (+ (`self.PlayerScore`) 1)))
  (`/Game/Blueprints/Widgets/UI/UMG_PlayerHUD.UpdatePlayerScore` (`/Game/Blueprints/BP_Paddle.PlayerUIRef` (`self.PlayerPaddle`)) _output_get)
  (set `self.LastScore` "NewEnumerator0")
  (`self.ResetTheBall`)
  (bind _isended (`self.IsGameEnded`))
  (if _isended
    (`self.GameEnded`)))

(fn `GameEnded`
  (locals (Looser :type String :default "You Loose!!") (Winner :type String :default "Winner!!!"))
  (bind _returnvalue (`GameplayStatics.GetPlayerController` 0))
  (bind _endmenu_uiref (`self.EndMenu_UIRef`))
  (bind _returnvalue_2 (`|CreateWidget` "/Game/Blueprints/Widgets/UI/UMG_EndMenu.UMG_EndMenu_C"))
  (bind _output_get (set `self.EndMenu_UIRef` _returnvalue_2))
  (`UserWidget.AddToViewport` _output_get 0)
  (`WidgetBlueprintLibrary.SetInputMode_UIOnlyEx` _returnvalue null)
  (set `PlayerController.bShowMouseCursor` true _returnvalue)
  (if (== (`self.AIScore`) (`self.MaxScore`))
    (`/Game/Blueprints/Widgets/UI/UMG_EndMenu.SetEndMessage` _endmenu_uiref (`local.Looser`))
    (else
      (`/Game/Blueprints/Widgets/UI/UMG_EndMenu.SetEndMessage` _endmenu_uiref (`local.Winner`)))))

(fn `InitLevelActors`
  (bind _returnvalue (`|SpawnActorFromClass` "/Game/Blueprints/BP_Ball.BP_Ball_C" (`KismetMathLibrary.Conv_VectorToTransform` (`self.BallStartLocation`)) "Undefined" "OverrideRootScale" null null))
  (set `self.TheBall` _returnvalue)
  (bind _outactors (`GameplayStatics.GetAllActorsOfClass` "/Game/Blueprints/BP_AIPaddle.BP_AIPaddle_C"))
  (bind _output_get (set `self.AIPaddle` (`|GetArrayItem` _outactors)))
  (`/Game/Blueprints/BP_AIPaddle.SetGameBallReference` _output_get (`self.TheBall`))
  (bind _outactors_2 (`GameplayStatics.GetAllActorsOfClass` "/Game/Blueprints/BP_Paddle.BP_Paddle_C"))
  (set `self.PlayerPaddle` (`|GetArrayItem` _outactors_2)))

(fn `IsGameEnded`
  (returns (IsEnded :type Boolean))
  (bind _maxscore (`self.MaxScore`))
  (if (== (`self.PlayerScore`) _maxscore)
    (return true)
    (elif (== _maxscore (`self.AIScore`))
      (return true)
      (else
        (return false)))))

(fn `LaunchTheBall`
  (params (YDirection :type "Float (double-precision)"))
  (`/Game/Blueprints/BP_Ball.FireInDirection` (`self.TheBall`) (`KismetMathLibrary.MakeVector` 0.0 YDirection)))

(fn `LaunchTheBallToAI`
  (`self.LaunchTheBall` 1.0))

(fn `LaunchTheBallToPlayer`
  (`self.LaunchTheBall` -1.0))

(fn `ResetTheBall`
  (bind _theball (`self.TheBall`))
  (`/Game/Blueprints/BP_Ball.StopMovement` _theball)
  (`self.K2_SetActorLocation` _theball (`self.BallStartLocation`) false false))

(fn `StarPlaying`
  (set `self.CurrentState` "NewEnumerator1")
  (if (`|EnumEquality` (`self.LastScore`) "NewEnumerator1")
    (`self.LaunchTheBallToAI`)
    (else
      (`self.LaunchTheBallToPlayer`))))

(fn `StartGame`
  (if (`self.IsFirstStart`)
    (`self.InitLevelActors`)
    (`self.StarPlaying`)
    (else
      (set `self.PlayerScore` 0)
      (set `self.AIScore` 0)
      (set `self.CurrentState` "NewEnumerator0")
      (`self.K2_SetActorLocation` (`self.AIPaddle`) (`self.AILocation`) false false)
      (`self.K2_SetActorLocation` (`self.PlayerPaddle`) (`self.PlayerLocation`) false false)
      (`self.StarPlaying`))))

(fn `UserConstructionScript`)